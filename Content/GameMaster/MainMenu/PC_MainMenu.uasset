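; Player controller for the main menu that shows the login widget on start, then swaps it for the main menu widget after a successful login.
; BeginPlay registers itself on the game instance, enables the cursor with Game and UI input, and binds to the game instance's login-completed delegate.
; A separate event hooks the game instance's create-completed delegate, but its session handler is empty.
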(event Custom|CE_CreateDelegate
  (params (sessionName :type Name) (bWasSuccessful :type Boolean)))

(event Custom|OnLoginCompleted
  (params (numOfPlayers :type Integer) (bWasSuccessful :type Boolean))
  (if bWasSuccessful
    (Development|PrintString (Utilities|String|ToString(Integer) numOfPlayers))
    (CallFunction|CECreateMainMenu)))

(event Custom|CE_CreateMainMenu
  (bind _wbp_login (Variables|Default|GetWBP_Login)
    (:then
      (Widget|RemovefromParent _wbp_login))
    (:else
      _))
  (bind _returnvalue (UserInterface|CreateWidget "/Game/Widgets/WBP_MainMenu.WBP_MainMenu_C" self))
  (bind _output_get (Variables|Default|SetWBP_MainMenu _returnvalue))
  (UserInterface|Viewport|AddtoViewport _output_get 0)
  (Input|SetInputModeGameandUI self _output_get "DoNotLock" false false))

(event Custom|CE_CreateResult
  (Class|EOSGameInstance|CreateCompletedDelegate (CallFunction|FlibGetGI) (delegate Custom|CE_CreateDelegate)))

(event EventBeginPlay
  (Variables|/Script/EOSFun.EOSGameInstance|SetRef_PCMainMenu (CallFunction|FlibGetGI) self)
  (Variables|Default|SetbShowMouseCursor true)
  (bind _returnvalue (UserInterface|CreateWidget "/Game/Widgets/WBP_Login.WBP_Login_C" self))
  (bind _output_get (Variables|Default|SetWBP_Login _returnvalue))
  (UserInterface|Viewport|AddtoViewport _output_get 0)
  (Input|SetInputModeGameandUI self _output_get "DoNotLock" false false)
  (Class|EOSGameInstance|LoginCompletedDelegate (CallFunction|FlibGetGI) (delegate Custom|OnLoginCompleted)))

(fn ConstructionScript)