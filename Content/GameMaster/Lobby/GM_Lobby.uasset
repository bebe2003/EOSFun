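; Lobby game mode Blueprint holding session-name plumbing, with an empty BeginPlay.
; OnSessionName prints the name and forwards it to the first player's PC_Lobby through CESetSessionName.
; The chain that copies the session name from game instance to game state and hooks OnSessionName to its replication is disconnected, so nothing in this graph triggers the handler.
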(event Custom|OnSessionName
  (params (SessionName :type String))
  (Development|PrintString (Utilities|String|ToString(Text) (Utilities|Text|FormatText "On session name replicated {name}" SessionName)))
  (bind _aspc_lobby (Utilities|Casting|CastToPC_Lobby (Game|GetPlayerController 0)))
  (Default|CESetSessionName _aspc_lobby SessionName)
  (Development|PrintString "Controller session name "))

(event EventBeginPlay)

(event EventTick
  (params (DeltaSeconds :type Float%20%28single-precision%29)))

(fn ConstructionScript)