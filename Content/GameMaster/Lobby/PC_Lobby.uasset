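; PC_Lobby is the player controller for the lobby, setting up its UI and showing the session name.
; On BeginPlay it registers itself with the game instance, shows the cursor, creates the WBP_LobbyLayout widget and switches input to Game and UI.
; It passes the game instance's current session name to the widget, and CE_SetSessionName forwards later name updates to it.
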(event Custom|CE_SetSessionName
  (params (SessionName :type String))
  (Default|CESetSessionName (Variables|Default|GetWBP_LobbyLayout) SessionName)
  (Development|PrintString "Set Session Successfully"))

(event EventBeginPlay
  (Variables|/Script/EOSFun.EOSGameInstance|SetRef_PCLobby (CallFunction|FlibGetGI) self)
  (Variables|Default|SetbShowMouseCursor true)
  (bind _returnvalue (UserInterface|CreateWidget "/Game/Widgets/WBP_LobbyLayout.WBP_LobbyLayout_C" self))
  (bind _output_get (Variables|Default|SetWBP_LobbyLayout _returnvalue))
  (UserInterface|Viewport|AddtoViewport _output_get 0)
  (Input|SetInputModeGameandUI self _output_get "DoNotLock" false false)
  (Default|CESetSessionName (Variables|Default|GetWBP_LobbyLayout) (Utilities|String|ToString(Name) (Class|EOSGameInstance|GetCurrentSessionName (CallFunction|FlibGetGI)))))

(fn ConstructionScript)